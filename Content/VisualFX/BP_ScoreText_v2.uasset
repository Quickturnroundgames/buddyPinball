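; BP_ScoreText_v2 is a floating score popup actor that shows a score increment as world-space text.
; On BeginPlay it sets the text from ScoreIncrement and falls back to its own world location if OriginPoint is zero.
; A timeline then drives text size and upward offset from that origin, while a parallel delay destroys the actor after LifeSpan.
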(event EventBeginPlay
  (Rendering|Components|TextRender|SetText (Variables|Default|GetScoreText) (Utilities|Text|ToText(String) (Utilities|String|Append (Utilities|String|ToString(Integer) (Variables|Default|GetscoreIncrement)) "")))
  (if (Math|Vector|NotEqual(Vector) (Variables|Default|GetoriginPoint) "0, 0, 0" 0.0001)
    _
    (else
      (Variables|Default|SetoriginPoint (Transformation|GetWorldLocation (Variables|Default|GetDefaultSceneRoot)))))
  (Utilities|FlowControl|Sequence
    (:then_0
      (Utilities|FlowControl|Delay (Variables|Default|GetlifeSpan))
      (Actor|DestroyActor))
    (:then_1
      (bind (_direction _sizealpha _locationalpha) (Timeline|PopTimeline Play)
        (:Update
          (Rendering|Components|TextRender|SetWorldSize (Variables|Default|GetScoreText) (* _sizealpha (Variables|Default|GettextSize)))
          (Transformation|SetWorldLocation (Variables|Default|GetDefaultSceneRoot) (+ (Variables|Default|GetoriginPoint) (Math|Vector|MakeVector 0.0 0.0 (* _locationalpha (Variables|Default|GetdistanceUpwards)))) false false))))))

(fn ConstructionScript)