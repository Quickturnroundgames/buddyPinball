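; BP_PointsHoleArea is a pinball points hole that holds a buddy, awards a streak of points, then launches it out.
; When a BP_BaseBuddy overlaps the trigger, it notifies the buddy and starts a delayed loop spawning one BP_ScoreText_v2 per streak step, each carrying the score increment.
; Once the loop completes, it releases the buddy using direction and force from LaunchDirectionArrow.
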(event OnComponentBeginOverlap(PointsAreaTrigger)
  (params (OverlappedComponent :type Primitive%20Component%20Object%20Reference) (OtherActor :type Actor%20Object%20Reference) (OtherComp :type Primitive%20Component%20Object%20Reference) (OtherBodyIndex :type Integer) (bFromSweep :type Boolean) (SweepResult :type Hit%20Result%20Structure%20%28by%20ref%29))
  ;[1 0 0] Comment
  (if (== "/Game/Character/BP_BaseBuddy.BP_BaseBuddy_C" (Utilities|GetClass OtherActor))
    (bind _asbp_base_buddy (Utilities|Casting|CastToBP_BaseBuddy OtherActor))
    (Variables|Default|SetBuddy _asbp_base_buddy)
    (Default|EnteredPointsHoleArea _asbp_base_buddy)
    (CallFunction|AcquirePoints)))

(event Custom|AcquirePoints
  (bind _defaultsceneroot (Variables|Default|GetDefaultSceneRoot))
  (bind _returnvalue (Transformation|GetWorldLocation _defaultsceneroot))
  (Utilities|ForLoopwithDelay 0 (- (Variables|Default|GetPointsStreak) 1) (Variables|Default|GetStreakDelay)
    (:loopBody
      (Game|SpawnActorfromClass "/Game/VisualFX/BP_ScoreText_v2.BP_ScoreText_v2_C" (Math|Transform|MakeTransform _returnvalue) "Undefined" 0 4.0 (+ _returnvalue "200.000000, 0, 0") 3e+02 (Variables|Default|GetPointsPerStreak) 1.0 0))
    (:completed
      (bind (_outdirection _outforce) (Default|GetData (Variables|Default|GetlaunchDirectionArrow)))
      (Default|LeavePointsHoleArea (Variables|Default|GetBuddy) _outdirection _outforce))))

(event EventBeginPlay)

(event Collision|EventActorBeginOverlap
  (params (OtherActor :type Actor%20Object%20Reference)))

(event EventTick
  (params (DeltaSeconds :type Float%20%28single-precision%29)))

(fn ConstructionScript)