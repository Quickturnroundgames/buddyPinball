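; BP_PortalEntrance is a pinball portal entrance that sends buddy balls to a linked PortalExit.
; When an actor of exactly the BP_BaseBuddy class overlaps the teleport trigger, it calls that buddy's EnteredPortal.
; The call passes travel time, the exit's location and speed, and whether the trip swaps sides, leaving the travel itself to the buddy.
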(event OnComponentBeginOverlap(TeleportTrigger)
  (params (OverlappedComponent :type Primitive%20Component%20Object%20Reference) (OtherActor :type Actor%20Object%20Reference) (OtherComp :type Primitive%20Component%20Object%20Reference) (OtherBodyIndex :type Integer) (bFromSweep :type Boolean) (SweepResult :type Hit%20Result%20Structure%20%28by%20ref%29))
  (if (== "/Game/Character/BP_BaseBuddy.BP_BaseBuddy_C" (Utilities|GetClass OtherActor))
    (bind _asbp_base_buddy (Utilities|Casting|CastToBP_BaseBuddy OtherActor))
    (Default|EnteredPortal _asbp_base_buddy (Variables|Default|GetTravelTime) self (Transformation|GetWorldLocation (Variables|/Script/Engine.Actor|GetRootComponent (Variables|Default|GetPortalExit))) (Variables|/Game/PinballsBPs/Portals/BP_PortalExit.BP_PortalExit_C|GetExitSpeed (Variables|Default|GetPortalExit)) (Variables|Default|GettakesToOtherSide))))

(fn ConstructionScript)