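; Pinball table Blueprint that coordinates play, routing finger input by pinball state to either the launch gauge or the hand flippers.
; While waiting, holds charge and release the launch hand, and taps can swap table side, splitter gate and camera.
; During play, input drives one or both flipper sides and nudges buddies.
; It also tracks multiplied score, timed combos, a post-launch redemption window and delayed gauge reset on ball out.
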(event Custom|StartFingerHold
  (params (isOnRightSide :type Boolean))
  ;[1 1 1] START FINGER LONG HOLD
  (switch Utilities|FlowControl|Switch|SwitchonEPinballState (Variables|Default|GetePinballState)
    (:NewEnumerator0
      (CallFunction|StartHandAnimation))))

(event Custom|LaunchBuddyFromHand
  ;[1 0 0.6058] GAUGE
  (Default|ReleaseGauge (Variables|Hands|GetLaunchHand)))

(event Custom|SetPinballState
  (params (pinballState :type EPinballState%20Enum :default "NewEnumerator0"))
  ;[1 1 1] SET PINBALL STATE
  (Variables|Default|SetePinballState pinballState))

(event Custom|StartFingerTap
  (params (IsOnRightSide :type Boolean))
  ;[1 1 1] START FINGER TAP
  (switch Utilities|FlowControl|Switch|SwitchonEPinballState (Variables|Default|GetePinballState)
    (:NewEnumerator1
      (if (Variables|Flippers|GetDoubleFlipper)
        (Utilities|FlowControl|Sequence
          (:then_0
            (for _array_element (Variables|Hands|GetHandR) :!label _label
              (Default|StartRotating _array_element)))
          (:then_1
            (for _array_element_2 (Variables|Hands|GetHandL) :!label _label_2
              (Default|StartRotating _array_element_2))))
        (elif IsOnRightSide
          (goto _label)
          (else
            (goto _label_2)))))))

(event Custom|ReleaseFingerHold
  (params (IsOnRightSide :type Boolean))
  ;[1 1 1] RELEASE FINGER HOLD
  (switch Utilities|FlowControl|Switch|SwitchonEPinballState (Variables|Default|GetePinballState)
    (:NewEnumerator0
      (CallFunction|LaunchBuddyfromHand))
    (:NewEnumerator1
      (if (Variables|Flippers|GetDoubleFlipper)
        (Utilities|FlowControl|Sequence
          (:then_0
            (for _array_element (Variables|Hands|GetHandR) :!label _label
              (Default|StopRotating _array_element)))
          (:then_1
            (for _array_element_2 (Variables|Hands|GetHandL) :!label _label_2
              (Default|StopRotating _array_element_2))))
        (elif IsOnRightSide
          (goto _label)
          (else
            (goto _label_2)))))))

(event Custom|ReleaseFingerTap
  (params (isOnRightSide :type Boolean))
  ;[1 1 1] RELEASE FINGER TAP
  (switch Utilities|FlowControl|Switch|SwitchonEPinballState (Variables|Default|GetePinballState)
    (:NewEnumerator0
      (if (Math|Boolean|NotEqual(Boolean) isOnRightSide (Variables|Default|GetisOnRightSide))
        (CallFunction|SwapTableSide)))
    (:NewEnumerator1
      (if (Variables|Flippers|GetDoubleFlipper)
        (Utilities|FlowControl|Sequence
          (:then_0
            (for _array_element (Variables|Hands|GetHandR) :!label _label
              (Default|StopRotating _array_element)))
          (:then_1
            (for _array_element_2 (Variables|Hands|GetHandL) :!label _label_2
              (Default|StopRotating _array_element_2))))
        (elif isOnRightSide
          (goto _label)
          (else
            (goto _label_2)))))))

(event Custom|StartHandAnimation
  ;[1 0 0.6058] GAUGE
  (Default|StartReadyLaunchBuddy (Variables|Hands|GetLaunchHand)))

(event Custom|SwapTableSide
  ;[1 1 1] SWAP SIDES
  (Default|FlipGate (Variables|Default|GetsplitterGate))
  (Variables|Default|SetisOnRightSide (not (Variables|Default|GetisOnRightSide)))
  (Default|SwapSide (Variables|Default|GetmainCamera)))

(event Custom|AddScore
  (params (ScoreIncrement :type Integer))
  (Variables|Default|SetTotalScore (+ (* ScoreIncrement (Variables|Default|GetScoreMultiplier)) (Variables|Default|GetTotalScore)))
  (Math|Integer|IncrementInt (Variables|Default|GetCurrentComboN)
    (:%20%20
      (Utilities|FlowControl|Sequence
        (:then_0
          (if (== (Variables|Default|GetCurrentComboN) (Variables|Default|GetUnstoppableComboN))
            (Audio|Components|Audio|Play (Variables|Default|GetUnstoppableComboAudio) 0.0)))
        (:then_1
          (Utilities|FlowControl|RetriggerableDelay (Variables|Default|GetComboTimer))
          (Variables|Default|SetCurrentComboN 0))))))

(event Custom|ResetGauge
  ;[1 1 1] RESET GAUGE
  (Utilities|FlowControl|Delay (Variables|Default|GetResetDelay))
  (Variables|Default|SetePinballState "NewEnumerator0")
  (Default|ResetGauge (Variables|Hands|GetLaunchHand)))

(event Custom|BuddyOut
  ;[1 1 1] ON BOTTOM TRIGGER BUDDY OVERLAP
  (CallFunction|ResetGauge))

(event Custom|BuddyLaunchedFromGauge
  ;[1 1 1] BUDDY LAUNCHED FROM GAUGE
  (Variables|Default|SetePinballState "NewEnumerator1")
  (CallFunction|StartRedemptionTimer))

(event Custom|NudgeBuddy
  (params (NudgeDirection :type Vector%202D%20Structure))
  (if (Utilities|Enum|Equal(Enum) (Variables|Default|GetePinballState) "NewEnumerator1")
    (for _array_element (Variables|Default|GetBuddies)
      (Default|NudgeinDirection _array_element NudgeDirection))))

(event Custom|StartRedemptionTimer
  ;[1 1 1] REDEMPTION TIMER
  (Variables|Default|SetredemptionOn true)
  (Utilities|FlowControl|RetriggerableDelay (Variables|Default|GetredemptionTime))
  (Variables|Default|SetredemptionOn false))

(fn ConstructionScript)