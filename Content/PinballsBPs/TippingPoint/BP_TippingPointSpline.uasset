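; Pinball Tipping Point spline actor that swings a snake head sideways by moving the last point of its spline.
; StartMoving and StopMoving set direction and state; while moving, Tick shifts that point along world Y at SelectorMoveSpeed, limited to MoveRange either side of its start.
; The head follows at its initial offset, and only the last spline mesh segment is reshaped to match.
; A leftover debug print shows the point's position during movement.
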(event Custom|StopMoving
  ;[1 1 1] MOVEMENT ON / OFF
  (Variables|Default|SetisMoving false))

(event Custom|StartMoving
  (params (moveRight :type Boolean))
  ;[1 1 1] MOVEMENT ON / OFF
  (Variables|Default|SetgoingRight moveRight)
  (Variables|Default|SetisMoving true))

(event EventTick
  (params (DeltaSeconds :type Float%20%28single-precision%29))
  (bind _selectormovespeed (Variables|Default|GetselectorMoveSpeed))
  (bind _moverange (Variables|Default|GetmoveRange))
  (bind _moverange_2 (Variables|Default|GetmoveRange))
  (bind _lastsplinepointindex (Variables|Default|GetlastSplinePointIndex))
  (bind _lastsplinepointindex_2 (Variables|Default|GetlastSplinePointIndex))
  (bind _lastsplinepointindex_3 (Variables|Default|GetlastSplinePointIndex))
  (bind _lastsplinepointinitiallocation (Variables|Default|GetlastSplinePointInitialLocation))
  (bind _spline (Variables|Default|GetSpline))
  (bind _lastsplinepointindex_4 (Variables|Default|GetlastSplinePointIndex))
  (bind _spline_2 (Variables|Default|GetSpline))
  (bind _lastsplinepointindex_5 (Variables|Default|GetlastSplinePointIndex))
  (bind _spline_3 (Variables|Default|GetSpline))
  (bind _lastsplinepointinitiallocation_2 (Variables|Default|GetlastSplinePointInitialLocation))
  (bind _spline_4 (Variables|Default|GetSpline))
  (bind _spline_5 (Variables|Default|GetSpline))
  (bind (_x _y _z) (Math|Vector|BreakVector _lastsplinepointinitiallocation_2))
  (bind _returnvalue (Spline|GetLocationatSplinePoint _spline _lastsplinepointindex_4 "World"))
  (bind _y_2 (Math|Vector|BreakVector _lastsplinepointinitiallocation))
  (bind _returnvalue_2 (- _lastsplinepointindex_3 1))
  (bind _returnvalue_3 (* DeltaSeconds _selectormovespeed))
  (bind _returnvalue_4 (Math|Vector|MakeVector 0.0 _returnvalue_3 0.0))
  (bind _y_3 (Math|Vector|BreakVector _returnvalue))
  (bind _returnvalue_5 (- _y_2 _y_3))
  ;[1 1 1] EVENT TICK
  (if (Variables|Default|GetisMoving)
    (Utilities|FlowControl|Sequence
      (:then_0
        (if (Variables|Default|GetgoingRight)
          (if (< _returnvalue_5 _moverange)
            (Spline|SetLocationatSplinePoint _spline_3 _lastsplinepointindex_5 (- _returnvalue _returnvalue_4) "World" true)
            (else
              (Spline|SetLocationatSplinePoint _spline_3 _lastsplinepointindex_5 (Math|Vector|MakeVector _x (- _y _moverange) _z) "World" true)))
          (elif (> _returnvalue_5 (* _moverange_2 -1.0))
            (Spline|SetLocationatSplinePoint _spline_5 _lastsplinepointindex_2 (+ _returnvalue _returnvalue_4) "World" true)
            (else
              (Spline|SetLocationatSplinePoint _spline_5 _lastsplinepointindex_2 (Math|Vector|MakeVector _x (+ _y _moverange_2) _z) "World" true)))))
      (:then_1
        (Transformation|SetWorldLocation (Variables|Default|GetSnakeHead) (+ (Spline|GetLocationatSplinePoint (Variables|Default|GetSpline) (Variables|Default|GetlastSplinePointIndex) "World") (Variables|Default|GetsnakeHeadOffset)) false false)
        (SplineMesh|SetStartandEnd (Variables|Default|GetlastSplineMeshComponent) (Spline|GetLocationatSplinePoint _spline_2 _returnvalue_2 "Local") (Spline|GetTangentatSplinePoint _spline_2 _returnvalue_2 "Local") (Spline|GetLocationatSplinePoint _spline_4 _lastsplinepointindex "Local") (Spline|GetTangentatSplinePoint _spline_4 _lastsplinepointindex "Local") true :!class /Script/Engine.SplineMeshComponent))
      (:then_2
        (Development|PrintString (Utilities|String|ToString(Vector) (Spline|GetLocationatSplinePoint (Variables|Default|GetSpline) (Variables|Default|GetlastSplinePointIndex) "Local")) true true "(R=0.000000,G=0.660000,B=1.000000,A=1.000000)" (Utilities|Time|GetWorldDeltaSeconds))))))

(event EventBeginPlay
  ;[1 0 0] BEGINPLAY
  (bind _output_get (Variables|Default|SetlastSplinePointIndex (- (Spline|GetNumberOfSplinePoints (Variables|Default|GetSpline)) 1)))
  (Variables|Default|SetsnakeHeadOffset (- (Transformation|GetWorldLocation (Variables|Default|GetSnakeHead)) (Spline|GetLocationatSplinePoint (Variables|Default|GetSpline) _output_get "World")))
  (Variables|Default|SetlastSplinePointInitialLocation (Spline|GetLocationatSplinePoint (Variables|Default|GetSpline) _output_get "World")))

(event Collision|EventActorBeginOverlap
  (params (OtherActor :type Actor%20Object%20Reference))
  (|CallParentFunction OtherActor) ; This node is disabled and will not be called.\nDrag off pins to build functionality.
)

(fn ConstructionScript
  (|CallParentFunction))