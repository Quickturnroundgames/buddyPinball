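; BP_TippingPointShelf is the moving shelf for Tipping Point, sliding back and forth along world X while active.
; A timeline alpha scaled by MoveAmount offsets the shelf from its BeginPlay location using swept moves.
; On each timeline finish, a FlipFlop swaps between reverse and play to loop the motion.
; StopMovement halts the timeline, and StartMovement picks the direction from the stored flip-flop state.
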(event Custom|StartMovement
  ;[0 0.9325 1] MOVEMENT
  (Variables|Default|SetisActive true)
  (if (stale _isa)
    (bind _movementalpha (Timeline|MovementTimeline Reverse)
      (:Update
        (Transformation|SetWorldLocation (Variables|Default|GetTippingPointShelf) (+ (Variables|Default|GetinitialLocation) (Math|Vector|MakeVector (* _movementalpha (Variables|Default|GetmoveAmount)) 0.0 0.0)) true false))
      (:Finished
        (bind _isa (Utilities|FlowControl|FlipFlop)
          (:A
            (Timeline|MovementTimeline Reverse))
          (:B
            (Timeline|MovementTimeline Play)))))
    (else
      (Timeline|MovementTimeline Play))))

(event Custom|StopMovement
  (Variables|Default|SetisActive false)
  ;[0 0.9325 1] MOVEMENT
  (bind _movementalpha (Timeline|MovementTimeline Stop)
    (:Update
      (Transformation|SetWorldLocation (Variables|Default|GetTippingPointShelf) (+ (Variables|Default|GetinitialLocation) (Math|Vector|MakeVector (* _movementalpha (Variables|Default|GetmoveAmount)) 0.0 0.0)) true false))
    (:Finished
      (bind _isa (Utilities|FlowControl|FlipFlop)
        (:A
          (Timeline|MovementTimeline Reverse))
        (:B
          (Timeline|MovementTimeline Play))))))

(event EventBeginPlay
  (Variables|Default|SetinitialLocation (Transformation|GetWorldLocation (Variables|Default|GetTippingPointShelf))))

(fn ConstructionScript)