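; BP_TippingPointGeneral coordinates the Tipping Point pinball minigame, linking the PinballTable, UI, MovingShelf and LaneSelector.
; An incoming buddy opens lane selection, with left/right input forwarded to the selector.
; Start requires exactly one active buddy, then moves the shelf under a retriggerable timer.
; Each unique buddy knocked out restarts that timer; expiry stops the shelf and ends the minigame after a short delay.
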(event Custom|Start
  (bind _pinballtable (Variables|Default|GetpinballTable))
  (bind _buddymanager (Variables|/Game/PinballsBPs/BP_PinballTable.BP_PinballTable_C|GetbuddyManager _pinballtable))
  ;[1 1 1] START
  (if (== 1 (Variables|/Game/PinballsBPs/BP_BuddiesManager.BP_BuddiesManager_C|GetnumActive (Variables|/Game/PinballsBPs/BP_PinballTable.BP_PinballTable_C|GetbuddyManager (Variables|Default|GetpinballTable))))
    (Variables|Default|SetbuddyOutCount 0)
    (Default|AddtoTippingPointList _buddymanager (Utilities|Array|Get(acopy) (Variables|/Game/PinballsBPs/BP_BuddiesManager.BP_BuddiesManager_C|GetactiveBuddies _buddymanager)))
    (Default|StartShelfMove (Variables|Default|GetUI))
    (Default|StartMovement (Variables|Default|GetmovingShelf))
    (Variables|Default|SetisMovingShelf true)
    (CallFunction|StartShelfMoveTimer)))

(event Custom|End
  ;[1 1 1] END
  (if (Variables|Default|GetisMovingShelf)
    (Default|StopMovement (Variables|Default|GetmovingShelf))
    (Default|OnShelfStop (Variables|Default|GetUI))
    (Utilities|FlowControl|Delay 2.0)
    (Variables|Default|SetisMovingShelf false)
    (Default|EndOfTippingPoint (Variables|Default|GetpinballTable))
    (Default|OnEnd (Variables|Default|GetUI))))

(event Custom|BuddyOut
  (params (buddyOutted :type BP%20Base%20Buddy%20Object%20Reference))
  ;[1 1 1] ON BUDDY OUT
  (if (not (Utilities|Array|ContainsItem (Variables|Default|GetbuddiesOuted) buddyOutted))
    (bind _result (Math|Integer|IncrementInt (Variables|Default|GetbuddyOutCount))
      (:%20%20
        (Utilities|Array|Add (Variables|Default|GetbuddiesOuted) buddyOutted)
        (CallFunction|StartShelfMoveTimer)
        (Default|OnBuddyOut (Variables|Default|GetUI) _result (Variables|Default|GetshelfTimer))))))

(event Custom|BuddyComingIn
  (params (timeForRelease :type Float%20%28single-precision%29))
  ;[1 1 1] WHEN BUDDY GOES IN SPLINE TO START
  (Default|StartOfTippingPoint (Variables|Default|GetpinballTable))
  (Default|StartLaneSelection (Variables|Default|GetUI) timeForRelease))

(event Custom|StartShelfMoveTimer
  ;[1 1 1] START MINIGAME TIMER
  (if (Variables|Default|GetisMovingShelf)
    (Utilities|FlowControl|RetriggerableDelay (Variables|Default|GetshelfTimer))
    (CallFunction|End)))

(event Custom|MoveRight
  (Default|StartMoving (Variables|Default|GetlaneSelector) true))

(event Custom|MoveLeft
  (Default|StartMoving (Variables|Default|GetlaneSelector) false))

(event Custom|StopMoving
  (Default|StopMoving (Variables|Default|GetlaneSelector)))

(event Custom|DropBuddyIntoLane)

(fn ConstructionScript)