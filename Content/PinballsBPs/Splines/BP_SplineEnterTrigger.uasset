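; BP_SplineEnterTrigger is a trigger that starts a pinball buddy following a spline.
; When its collision component is overlapped by an actor whose class is exactly BP_BaseBuddy, it checks the buddy mesh's vertical velocity.
; If the Z velocity is zero or upward, it calls StartSplineFollow on its Spline reference, then Activated, which is empty here.
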(event OnComponentBeginOverlap(CollisionComponent)
  (params (OverlappedComponent :type Primitive%20Component%20Object%20Reference) (OtherActor :type Actor%20Object%20Reference) (OtherComp :type Primitive%20Component%20Object%20Reference) (OtherBodyIndex :type Integer) (bFromSweep :type Boolean) (SweepResult :type Hit%20Result%20Structure%20%28by%20ref%29))
  (if (== "/Game/Character/BP_BaseBuddy.BP_BaseBuddy_C" (Utilities|GetClass OtherActor))
    (bind _asbp_base_buddy (Utilities|Casting|CastToBP_BaseBuddy OtherActor))
    (if (>= (.Z (Math|Vector|BreakVector (Transformation|GetComponentVelocity (Variables|/Script/Engine.Character|GetMesh _asbp_base_buddy)))) 0.0)
      (Default|StartSplineFollow (Variables|Default|GetSpline) _asbp_base_buddy)
      (CallFunction|Activated))))

(fn ConstructionScript)

(fn Activated)