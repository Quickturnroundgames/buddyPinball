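; BP_ArrowForDirection is a pinball helper actor that supplies a launch direction and expeller force.
; GetData flattens its Arrow component's forward vector onto the YZ plane and normalizes it.
; It then rotates that vector around the X axis by a random angle within RandomDegreeRange, centred on the arrow, and returns it with ExpellerForce.
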(fn ConstructionScript)

(fn GetData
  (bind _arrow (Variables|Default|GetArrow))
  (bind _randomdegreerange (Variables|Default|GetRandomDegreeRange))
  (bind _returnvalue (Math|Vector|GetForwardVector _arrow))
  (bind _returnvalue_2 (* _randomdegreerange 0.5))
  (bind (_x _y _z) (Math|Vector|BreakVector _returnvalue))
  (return (Math|Vector|RotateVectorAroundAxis (Math|Vector|Normalize (Math|Vector|MakeVector 0.0 _y _z)) (Math|Random|RandomFloatinRange _returnvalue_2 (* _returnvalue_2 -1.0)) "1.000000,0.000000, 0") (Variables|Default|GetExpellerForce)))