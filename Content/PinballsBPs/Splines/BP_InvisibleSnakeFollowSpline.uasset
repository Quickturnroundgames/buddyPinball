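; BP_InvisibleSnakeFollowSpline is a pinball spline actor that carries a Buddy along its path and launches it out at the end.
; StartSplineFollow hands the Buddy itself, its speed, and the direction and force read from SplineExit, leaving the movement to the Buddy's FollowGaugeSpline.
; PlaySplineEndFX briefly activates the optional PooFX particles, using a playing flag to ignore repeat calls until they stop.
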(event Custom|StartSplineFollow
  (params (Buddy :type BP%20Base%20Buddy%20Object%20Reference))
  (bind (_outdirection _outforce) (Default|GetData (Variables|Default|GetSplineExit)))
  (Default|FollowGaugeSpline Buddy self (Variables|Default|GetSplineSpeed) _outdirection _outforce))

(event Custom|PlaySplineEndFX
  (bind _poofx (Variables|Default|GetPooFX))
  (bind _particlesystemcomponent (Variables|/Script/Engine.Emitter|GetParticleSystemComponent _poofx))
  ;[1 1 1] POO FX
  (Utilities|IsValid (Variables|Default|GetPooFX)
    (:Is%20Valid
      (if (not (Variables|Default|GetIsPlayingFX))
        (Variables|Default|SetIsPlayingFX true)
        (Components|Activation|Activate _particlesystemcomponent true)
        (Utilities|FlowControl|RetriggerableDelay 0.5)
        (Components|Activation|Deactivate _particlesystemcomponent)
        (Variables|Default|SetIsPlayingFX false)))))

(fn ConstructionScript)