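; Hand actor for a pinball game that swings its Wrist component on demand, similar to a flipper.
; BeginPlay caches the wrist's initial relative rotation as the rest pose.
; StartRotating plays a timeline whose alpha scales RotateDegrees into a pitch offset combined with that rest rotation.
; StopRotating reverses the same timeline, easing the wrist back from wherever it is.
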(event Custom|StartRotating
  (bind _rotatealpha (Timeline|RotateTimeline Play)
    (:Update
      (Transformation|SetRelativeRotation (Variables|Default|GetWrist) (Math|Rotator|CombineRotators (Variables|Default|GetInitialRotation) (Math|Rotator|MakeRotator 0.0 (* _rotatealpha (Variables|Default|GetRotateDegrees)) 0.0)) false false))))

(event Custom|StopRotating
  (bind _rotatealpha (Timeline|RotateTimeline Reverse)
    (:Update
      (Transformation|SetRelativeRotation (Variables|Default|GetWrist) (Math|Rotator|CombineRotators (Variables|Default|GetInitialRotation) (Math|Rotator|MakeRotator 0.0 (* _rotatealpha (Variables|Default|GetRotateDegrees)) 0.0)) false false))))

(event EventBeginPlay
  ;[0.3427 0 0.009388] Comment
  (Variables|Default|SetInitialRotation (Variables|/Script/Engine.SceneComponent|GetRelativeRotation (Variables|Default|GetWrist))))

(fn ConstructionScript)