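; BP_LaunchHand is a pinball-style launcher hand that holds a Buddy character and flings it on release.
; On hold, a timeline lowers the hand from its starting position; on release, a second timeline raises it, then calls LaunchFromPinball with force scaled by the pull-down alpha.
; Tick and both timelines pin the Buddy's capsule to the BuddyPos component, offset by its half height, until launch.
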(event Custom|StartReadyLaunchBuddy
  ;[0.04722 1 0] ON START HOLD (READY LAUNCH)
  (if (and (not (Variables|Animation|GetIsReadyingLaunch)) (not (Variables|Animation|GetHasLaunchedBuddy)))
    (Variables|Animation|SetIsReadyingLaunch true)
    (bind _handdownalpha (Timeline|ReadyLaunchTimeline PlayFromStart)
      (:Update
        (if (Variables|Animation|GetIsReadyingLaunch)
          (Transformation|SetWorldLocation (Variables|Default|GetDefaultSceneRoot) (- (Variables|Animation|GetInitialHandPos) (Math|Vector|MakeVector 0.0 0.0 (* _handdownalpha (Variables|Animation|GetDownDistance)))) false true)
          (if (Variables|Animation|GetIsReadyingLaunch)
            (Transformation|SetWorldLocation (Variables|/Script/Engine.Character|GetCapsuleComponent (Variables|Default|GetBuddy)) (+ (Math|Vector|MakeVector 0.0 0.0 (Variables|Default|GetBuddyHalfHeight)) (Transformation|GetWorldLocation (Variables|Default|GetBuddyPos))) false true)))))))

(event Custom|LaunchBuddy
  (params (LaunchForce :type Float%20%28single-precision%29))
  ;[0.4052 0.1194 0] ON RELEASE (LAUNCH)
  (Utilities|FlowControl|Sequence
    (:then_0
      ;[0.04722 1 0] ON START HOLD (READY LAUNCH)
      (bind _handdownalpha (Timeline|ReadyLaunchTimeline Stop)
        (:Update
          (if (Variables|Animation|GetIsReadyingLaunch)
            (Transformation|SetWorldLocation (Variables|Default|GetDefaultSceneRoot) (- (Variables|Animation|GetInitialHandPos) (Math|Vector|MakeVector 0.0 0.0 (* _handdownalpha (Variables|Animation|GetDownDistance)))) false true)
            (if (Variables|Animation|GetIsReadyingLaunch)
              (Transformation|SetWorldLocation (Variables|/Script/Engine.Character|GetCapsuleComponent (Variables|Default|GetBuddy)) (+ (Math|Vector|MakeVector 0.0 0.0 (Variables|Default|GetBuddyHalfHeight)) (Transformation|GetWorldLocation (Variables|Default|GetBuddyPos))) false true))))))
    (:then_1
      (Variables|Animation|SetHasLaunchedBuddy true)
      (Variables|Animation|SetIsReadyingLaunch true))
    (:then_2
      (bind _handupalpha (Timeline|ReleaseHandTimeline PlayFromStart)
        (:Update
          (Transformation|SetWorldLocation (Variables|Default|GetDefaultSceneRoot) (+ (Variables|Animation|GetInitialHandPos) (Math|Vector|MakeVector 0.0 0.0 (* _handupalpha (Variables|Animation|GetDownDistance)))) false true)
          (Transformation|SetWorldLocation (Variables|/Script/Engine.Character|GetCapsuleComponent (Variables|Default|GetBuddy)) (+ (Math|Vector|MakeVector 0.0 0.0 (Variables|Default|GetBuddyHalfHeight)) (Transformation|GetWorldLocation (Variables|Default|GetBuddyPos))) false true))
        (:Finished
          (Default|LaunchfromPinball (Variables|Default|GetBuddy) (* _handdownalpha LaunchForce)))))))

(event EventBeginPlay
  ;[0.3427 0 0.009388] BEGIN PLAY
  (Variables|Animation|SetInitialHandPos (Transformation|GetWorldLocation (Variables|Default|GetDefaultSceneRoot)))
  (bind _halfheight (Default|GetHalfHeight (Variables|Default|GetBuddy)))
  (Variables|Default|SetBuddyHalfHeight _halfheight)
  (Transformation|SetWorldLocation (Variables|/Script/Engine.Character|GetCapsuleComponent (Variables|Default|GetBuddy)) (Transformation|GetWorldLocation (Variables|Default|GetBuddyPos)) false true))

(event EventTick
  (params (DeltaSeconds :type Float%20%28single-precision%29))
  ;[0.3427 0 0.009388] EVEN TICK
  (if (and (not (Variables|Animation|GetIsReadyingLaunch)) (not (Variables|Animation|GetHasLaunchedBuddy)))
    (Transformation|SetWorldLocation (Variables|/Script/Engine.Character|GetCapsuleComponent (Variables|Default|GetBuddy)) (+ (Math|Vector|MakeVector 0.0 0.0 (Variables|Default|GetBuddyHalfHeight)) (Transformation|GetWorldLocation (Variables|Default|GetBuddyPos))) false true)))

(fn ConstructionScript)

(fn SetBuddy
  (params (Buddy :type BP%20Base%20Buddy%20Object%20Reference))
  (Variables|Default|SetBuddy Buddy))