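; BP_TippingPointShelf is a shelf that slides back and forth along the X axis, starting on BeginPlay.
; A timeline's alpha, scaled by MoveAmount and delta seconds, feeds a swept world offset on the shelf every update.
; When the timeline finishes, a FlipFlop alternates reversing and replaying it, and its state also switches the movement's sign.
; Tick checks IsActive but does nothing.
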(event Custom|StartMovement
  (bind _returnvalue (Utilities|Time|GetWorldDeltaSeconds))
  ;[0 0.9325 1] MOVEMENT
  (Variables|Default|SetisActive true)
  (bind _movementalpha (Timeline|MovementTimeline Play)
    (:Update
      (if (stale _isa)
        (Transformation|AddWorldOffset (Variables|Default|GetTippingPointShelf) (Math|Vector|MakeVector (* _movementalpha (Variables|Default|GetmoveAmount) _returnvalue) 0.0 0.0) true false)
        (else
          (Transformation|AddWorldOffset (Variables|Default|GetTippingPointShelf) (Math|Vector|MakeVector (* _movementalpha (Variables|Default|GetmoveAmount) -1.0 _returnvalue) 0.0 0.0) true false))))
    (:Finished
      (bind _isa (Utilities|FlowControl|FlipFlop)
        (:A
          (Timeline|MovementTimeline ReverseFromEnd))
        (:B
          (Timeline|MovementTimeline PlayFromStart))))))

(event EventBeginPlay
  (CallFunction|StartMovement))

(event EventTick
  (params (DeltaSeconds :type Float%20%28single-precision%29))
  (if (Variables|Default|GetisActive)
    _))

(fn ConstructionScript)