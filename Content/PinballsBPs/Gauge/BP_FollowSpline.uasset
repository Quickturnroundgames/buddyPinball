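; Spline track actor in the pinball gauge system that carries a Buddy along its path and supplies its exit launch.
; The construction script builds a forward-X spline mesh segment between each pair of spline points, matching their local positions and tangents.
; StartSplineFollow reads direction and force from SplineExit and passes them with itself to the Buddy's FollowGaugeSpline, which handles the movement.
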(event Custom|StartSplineFollow
  (params (Buddy :type BP%20Base%20Buddy%20Object%20Reference))
  (bind (_outdirection _outforce) (Default|GetData (Variables|Default|GetSplineExit)))
  (Default|FollowGaugeSpline Buddy self 1.0 _outdirection _outforce))

(fn ConstructionScript
  (bind _spline (Variables|Default|GetSpline))
  (bind _spline_2 (Variables|Default|GetSpline))
  (for _index (range 0 (- (Spline|GetNumberOfSplinePoints (Variables|Default|GetSpline)) 2))
    (bind _returnvalue (AddComponent|AddSplineMeshComponent false))
    (SplineMesh|SetForwardAxis _returnvalue "X" true)
    (SplineMesh|SetStartandEnd _returnvalue (Spline|GetLocationatSplinePoint _spline _index "Local") (Spline|GetTangentatSplinePoint _spline _index "Local") (Spline|GetLocationatSplinePoint _spline_2 (+ _index 1) "Local") (Spline|GetTangentatSplinePoint _spline_2 (+ _index 1) "Local") true :!class /Script/Engine.SplineMeshComponent)
    (Collision|SetCollisionEnabled (Variables|Default|GetSpline) "NoCollision")))