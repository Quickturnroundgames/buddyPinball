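; BP_LaunchSpline is a spline track that sends BP_BaseBuddy actors along the pinball launch gauge.
; The construction script builds the visible track, adding one spline mesh per segment between points, matched to the spline's positions and tangents.
; When an actor of exactly the BP_BaseBuddy class overlaps the trigger sphere, the Blueprint calls FollowGaugeSpline on it, leaving the movement to the buddy.
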(event OnComponentBeginOverlap(Sphere)
  (params (OverlappedComponent :type Primitive%20Component%20Object%20Reference) (OtherActor :type Actor%20Object%20Reference) (OtherComp :type Primitive%20Component%20Object%20Reference) (OtherBodyIndex :type Integer) (bFromSweep :type Boolean) (SweepResult :type Hit%20Result%20Structure%20%28by%20ref%29))
  (if (== "/Game/Character/BP_BaseBuddy.BP_BaseBuddy_C" (Utilities|GetClass OtherActor))
    (bind _asbp_base_buddy (Utilities|Casting|CastToBP_BaseBuddy OtherActor))
    (Default|FollowGaugeSpline _asbp_base_buddy)))

(fn ConstructionScript
  (bind _spline (Variables|Default|GetSpline))
  (bind _spline_2 (Variables|Default|GetSpline))
  (for _index (range 0 (- (Spline|GetNumberOfSplinePoints (Variables|Default|GetSpline)) 2))
    (bind _returnvalue (AddComponent|AddSplineMeshComponent false))
    (SplineMesh|SetForwardAxis _returnvalue "X" true)
    (SplineMesh|SetStartandEnd _returnvalue (Spline|GetLocationatSplinePoint _spline _index "Local") (Spline|GetTangentatSplinePoint _spline _index "Local") (Spline|GetLocationatSplinePoint _spline_2 (+ _index 1) "Local") (Spline|GetTangentatSplinePoint _spline_2 (+ _index 1) "Local") true :!class /Script/Engine.SplineMeshComponent)
    (Collision|SetCollisionEnabled (Variables|Default|GetSpline) "NoCollision")))