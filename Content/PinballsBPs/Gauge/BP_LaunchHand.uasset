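; Pinball launch gauge: a hand that lowers while charging and springs back up to launch the Buddy into the pinball table.
; A state enum drives the flow, with Tick and timeline updates pinning the Buddy's capsule to the hand.
; Release reverses the timeline at a clamped speed based on pull depth.
; When the timeline finishes, sufficient speed launches the Buddy and notifies PinballTable; otherwise the gauge returns to Waiting.
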(event Custom|StartReadyLaunchBuddy
  ;[0.04722 1 0] ON START HOLD (READY LAUNCH)
  (if (Utilities|Enum|Equal(Enum) (Variables|Animation|GeteGaugeState) "NewEnumerator1")
    (Variables|Animation|SeteGaugeState "NewEnumerator2")
    (Components|Timeline|SetPlayRate (Variables|Default|GetHandMoveTimeline) 1.0)
    (bind _handposalpha (Timeline|HandMoveTimeline Play)
      (:Update
        (switch Utilities|FlowControl|Switch|SwitchonEGaugeState (Variables|Animation|GeteGaugeState)
          (:NewEnumerator2
            _)
          (:NewEnumerator3
            _))
        (Utilities|FlowControl|Sequence
          (:then_0
            (Transformation|SetWorldLocation (Variables|Default|GetDefaultSceneRoot) (- (Variables|Animation|GetInitialHandPos) (Math|Vector|MakeVector 0.0 0.0 (* _handposalpha (Variables|Animation|GetDownDistance)))) false true))
          (:then_1
            (Transformation|SetWorldLocation (Variables|/Script/Engine.Character|GetCapsuleComponent (Variables|Default|GetBuddy)) (+ (Math|Vector|MakeVector 0.0 0.0 (Variables|Default|GetBuddyHalfHeight)) (Transformation|GetWorldLocation (Variables|Default|GetBuddyPos))) false true))))
      (:Finished
        (CallFunction|CheckifCanLaunch)))))

(event Custom|ReleaseGauge
  ;[0.4052 0.1194 0] ON RELEASE (LAUNCH)
  (Utilities|FlowControl|Sequence
    (:then_0
      (Variables|Animation|SeteGaugeState "NewEnumerator3"))
    (:then_1
      (bind _output_get (Variables|Default|SetupSpeed (Math|Float|Clamp(Float) (* (stale _handposalpha) (Variables|Default|GetgaugeSpeed)) 1.0 12.0)))
      (Components|Timeline|SetPlayRate (Variables|Default|GetHandMoveTimeline) _output_get))
    (:then_2
      (bind _handposalpha (Timeline|HandMoveTimeline Reverse)
        (:Update
          (switch Utilities|FlowControl|Switch|SwitchonEGaugeState (Variables|Animation|GeteGaugeState)
            (:NewEnumerator2
              _)
            (:NewEnumerator3
              _))
          (Utilities|FlowControl|Sequence
            (:then_0
              ;[0.04722 1 0] ON START HOLD (READY LAUNCH)
              (Transformation|SetWorldLocation (Variables|Default|GetDefaultSceneRoot) (- (Variables|Animation|GetInitialHandPos) (Math|Vector|MakeVector 0.0 0.0 (* _handposalpha (Variables|Animation|GetDownDistance)))) false true))
            (:then_1
              (Transformation|SetWorldLocation (Variables|/Script/Engine.Character|GetCapsuleComponent (Variables|Default|GetBuddy)) (+ (Math|Vector|MakeVector 0.0 0.0 (Variables|Default|GetBuddyHalfHeight)) (Transformation|GetWorldLocation (Variables|Default|GetBuddyPos))) false true))))
        (:Finished
          (CallFunction|CheckifCanLaunch))))))

(event Custom|ResetGauge
  ;[1 1 1] RESET GAUGE
  (Variables|Animation|SeteGaugeState "NewEnumerator1")
  (Default|TurnRagdollOFF (Variables|Default|GetBuddy) "NewEnumerator0")
  (Transformation|SetWorldLocation (Variables|/Script/Engine.Character|GetCapsuleComponent (Variables|Default|GetBuddy)) (Transformation|GetWorldLocation (Variables|Default|GetBuddyPos)) false true))

(event Custom|CheckIfCanLaunch
  ;[1 1 1] CHECK IF CAN LAUNCH
  (if (>= (Variables|Default|GetupSpeed) 4.0)
    (Utilities|FlowControl|Sequence
      (:then_1
        (Variables|Animation|SeteGaugeState "NewEnumerator0")
        (Default|BuddyLaunchedfromGauge (Variables|Default|GetpinballTable))
        (Default|LaunchfromPinball (Variables|Default|GetBuddy) (* (Variables|Default|GetupSpeed) (Variables|Default|GetlaunchForce)))))
    (else
      (Variables|Animation|SeteGaugeState "NewEnumerator1"))))

(event EventBeginPlay
  ;[0.3427 0 0.009388] BEGIN PLAY
  (Variables|Animation|SetInitialHandPos (Transformation|GetWorldLocation (Variables|Default|GetDefaultSceneRoot)))
  (bind _halfheight (Default|GetHalfHeight (Variables|Default|GetBuddy)))
  (Variables|Default|SetBuddyHalfHeight _halfheight)
  (Transformation|SetWorldLocation (Variables|/Script/Engine.Character|GetCapsuleComponent (Variables|Default|GetBuddy)) (Transformation|GetWorldLocation (Variables|Default|GetBuddyPos)) false true)
  (Variables|Animation|SeteGaugeState "NewEnumerator1"))

(event EventTick
  (params (DeltaSeconds :type Float%20%28single-precision%29))
  ;[0.3427 0 0.009388] EVEN TICK
  (Utilities|FlowControl|Sequence
    (:then_2
      (switch Utilities|FlowControl|Switch|SwitchonEGaugeState (Variables|Animation|GeteGaugeState)
        (:NewEnumerator1
          _)
        (:NewEnumerator2
          _)
        (:NewEnumerator3
          _))
      (Transformation|SetWorldLocation (Variables|/Script/Engine.Character|GetCapsuleComponent (Variables|Default|GetBuddy)) (+ (Math|Vector|MakeVector 0.0 0.0 (Variables|Default|GetBuddyHalfHeight)) (Transformation|GetWorldLocation (Variables|Default|GetBuddyPos))) false true))))

(fn ConstructionScript)

(fn SetBuddy
  (params (Buddy :type BP%20Base%20Buddy%20Object%20Reference))
  (Variables|Default|SetBuddy Buddy))