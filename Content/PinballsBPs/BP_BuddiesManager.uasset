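; Manager for pinball buddies that tracks them across active, inactive and tipping point lists.
; Events move buddies between lists while keeping an active count, promoting the first inactive one below the maximum; SpawnNewOnGauge does so only when none are active.
; PlaceBuddy switches a buddy to ragdoll and teleports its mesh to a location.
; Tick prints the active count for debugging.
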(event Custom|SpawnNewOnGauge
  ;[1 1 1] SPAWN ON GAUGE
  (if (== (Variables|Default|GetnumActive) 0)
    (CallFunction|AddtoActivefromInactive)))

(event Custom|PlaceBuddy
  (params (location :type Vector%20%28by%20ref%29) (buddy :type BP%20Base%20Buddy%20Object%20Reference%20%28by%20ref%29))
  ;[1 1 1] PLACE BUDDY
  (Default|TurnRagdollON buddy)
  (Transformation|SetWorldLocation (Variables|/Script/Engine.Character|GetMesh buddy) location false true))

(event Custom|RemoveFromActive
  (params (buddy :type BP%20Base%20Buddy%20Object%20Reference%20%28by%20ref%29))
  ;[1 1 1] REMOVE FROM ACTIVE
  (Utilities|Array|RemoveItem (Variables|Default|GetactiveBuddies) buddy)
  (Math|Integer|DecrementInt (Variables|Default|GetnumActive)))

(event Custom|AddToActiveFromInactive
  (bind _inactivebuddies (Variables|Default|GetinactiveBuddies))
  (bind _output (Utilities|Array|Get(acopy) _inactivebuddies))
  ;[1 1 1] ADD TO ACTIVE FROM INACTIVE
  (if (!= (Variables|Default|GetnumActive) (Variables|Default|GetmaxNumActive))
    (CallFunction|AddtoActive _output)
    (Utilities|Array|RemoveItem _inactivebuddies _output)))

(event Custom|AddToTippingPointList
  (params (buddy :type BP%20Base%20Buddy%20Object%20Reference%20%28by%20ref%29))
  ;[1 1 1] ADD TO TIPPING POINT LIST
  (Utilities|Array|Add (Variables|Default|GettippingPointBuddies) buddy)
  (CallFunction|RemovefromActive buddy))

(event Custom|AddToActiveFromTippingPoint
  (params (buddy :type BP%20Base%20Buddy%20Object%20Reference%20%28by%20ref%29))
  ;[1 1 1] REMOVE FROM TIPPING POINT LIST
  (Utilities|Array|RemoveItem (Variables|Default|GettippingPointBuddies) buddy)
  (CallFunction|AddtoActive buddy))

(event Custom|AddToActive
  (params (buddy :type BP%20Base%20Buddy%20Object%20Reference%20%28by%20ref%29))
  ;[1 1 1] ADD TO ACTIVE
  (Utilities|Array|Add (Variables|Default|GetactiveBuddies) buddy)
  (Math|Integer|IncrementInt (Variables|Default|GetnumActive)))

(event EventBeginPlay
  ;[1 1 1] DEBUG ONLY PLES REMOVE
)

(event EventTick
  (params (DeltaSeconds :type Float%20%28single-precision%29))
  ;[1 1 1] DEBUG ONLY PLES REMOVE
  (Development|PrintString (Utilities|String|ToString(Integer) (Variables|Default|GetnumActive)) true true "(R=0.000000,G=0.660000,B=1.000000,A=1.000000)" DeltaSeconds))

(fn ConstructionScript)