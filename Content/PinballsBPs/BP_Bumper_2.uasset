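; Pinball bumper that reacts when a BP_BaseBuddy hits its collider, awarding score and knocking the buddy away.
; A WasHitRecently flag with a HitDelay cooldown gates the sound and the PinballTable score increase.
; Every hit, even during cooldown, applies BumperForce along the direction from ArrowForDirection and spawns a BP_ScoreText at the mesh location showing the increment.
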(event OnComponentBeginOverlap(BumperCollider)
  (params (OverlappedComponent :type Primitive%20Component%20Object%20Reference) (OtherActor :type Actor%20Object%20Reference) (OtherComp :type Primitive%20Component%20Object%20Reference) (OtherBodyIndex :type Integer) (bFromSweep :type Boolean) (SweepResult :type Hit%20Result%20Structure%20%28by%20ref%29)))

(event OnComponentHit(BumperCollider)
  (params (HitComponent :type Primitive%20Component%20Object%20Reference) (OtherActor :type Actor%20Object%20Reference) (OtherComp :type Primitive%20Component%20Object%20Reference) (NormalImpulse :type Vector :default "0, 0, 0") (Hit :type Hit%20Result%20Structure%20%28by%20ref%29))
  (bind _staticmeshcomponent (Variables|Debug|GetStaticMeshComponent))
  (bind _returnvalue (Transformation|GetWorldLocation _staticmeshcomponent))
  (if (== "/Game/Character/BP_BaseBuddy.BP_BaseBuddy_C" (Utilities|GetClass OtherActor))
    (Utilities|FlowControl|Sequence
      (:then_0
        (if (not (Variables|HitDelay|GetWasHitRecently))
          (Variables|HitDelay|SetWasHitRecently true)
          (Audio|Components|Audio|Play (Variables|Default|GetSoundFX) 0.0)
          (Default|AddScore (Variables|Default|GetPinballTable) (Variables|Default|GetScoreIncrement))
          (Utilities|FlowControl|Delay (Variables|HitDelay|GetHitDelay))
          (Variables|HitDelay|SetWasHitRecently false)))
      (:then_2
        (bind _outdirection (Default|GetData (Variables|Default|GetArrowForDirection)))
        (bind _asbp_base_buddy (Utilities|Casting|CastToBP_BaseBuddy OtherActor))
        (Default|BumperForce _asbp_base_buddy (Variables|Default|GetBumperForce) _outdirection))
      (:then_3
        (Game|SpawnActorfromClass "/Game/VisualFX/BP_ScoreText.BP_ScoreText_C" (Math|Transform|MakeTransform _returnvalue) "Undefined" 0 0.0 _returnvalue 2e+02 (Variables|Default|GetScoreIncrement) 0)))))

(fn ConstructionScript)