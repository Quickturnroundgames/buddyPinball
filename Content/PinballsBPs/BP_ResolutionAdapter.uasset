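; BP_ResolutionAdapter is an actor that adapts the pinball scene to the screen's aspect ratio at startup.
; Shortly after BeginPlay, it computes the viewport aspect ratio and repositions the LeftPoint and RightPoint actors along world X with a shared logarithmic formula, preserving their Y and Z.
; It then calls AdjustResolution on MainCamera so the camera can update.
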(event EventBeginPlay
  (bind _returnvalue (Viewport|GetViewportSize))
  (bind _leftpoint (Variables|Default|GetleftPoint))
  (bind _rightpoint (Variables|Default|GetrightPoint))
  (bind (_x _y) (Math|Vector2D|BreakVector2D _returnvalue))
  (bind _rootcomponent (Variables|/Script/Engine.Actor|GetRootComponent _rightpoint))
  (bind _rootcomponent_2 (Variables|/Script/Engine.Actor|GetRootComponent _leftpoint))
  (bind _returnvalue_2 (Transformation|GetWorldLocation _rootcomponent))
  (bind _returnvalue_3 (Transformation|GetWorldLocation _rootcomponent_2))
  (bind (_x_2 _y_2 _z) (Math|Vector|BreakVector _returnvalue_2))
  (bind (_x_3 _y_3 _z_2) (Math|Vector|BreakVector _returnvalue_3))
  (Utilities|FlowControl|Delay 0.2)
  (Variables|Default|SetaspectRatio (/ _x _y))
  (Transformation|SetWorldLocation _rootcomponent_2 (Math|Vector|MakeVector (+ (* (Variables|Default|GetaspectRatio) 4e+03 (Math|Float|Log (Variables|Default|GetaspectRatio) 1e+01)) 4e+03) _y_3 _z_2) false false)
  (Transformation|SetWorldLocation _rootcomponent (Math|Vector|MakeVector (+ (* (Variables|Default|GetaspectRatio) 4e+03 (Math|Float|Log (Variables|Default|GetaspectRatio) 1e+01)) 4e+03) _y_2 _z) false false)
  (Default|AdjustResolution (Variables|Default|GetmainCamera)))

(event Collision|EventActorBeginOverlap
  (params (OtherActor :type Actor%20Object%20Reference)))

(fn ConstructionScript)