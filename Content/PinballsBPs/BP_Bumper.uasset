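; BP_Bumper is a pinball bumper that knocks buddy actors away and awards score when they hit it.
; On a hit from an exact BP_BaseBuddy class, it calls BumperForce along the inverted hit normal, plays a sound and adds points to PinballTable.
; It also spawns a BP_ScoreText at the bumper showing the increment.
; A WasHitRecently flag, cleared after HitDelay, debounces repeated hits.
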(event Collision|EventHit
  (params (MyComp :type Primitive%20Component%20Object%20Reference) (Other :type Actor%20Object%20Reference) (OtherComp :type Primitive%20Component%20Object%20Reference) (bSelfMoved :type Boolean) (HitLocation :type Vector :default "0, 0, 0") (HitNormal :type Vector :default "0, 0, 0") (NormalImpulse :type Vector :default "0, 0, 0") (Hit :type Hit%20Result%20Structure%20%28by%20ref%29))
  (bind _staticmeshcomponent (Variables|Debug|GetStaticMeshComponent))
  (bind _returnvalue (Transformation|GetWorldLocation _staticmeshcomponent))
  (if (== "/Game/Character/BP_BaseBuddy.BP_BaseBuddy_C" (Utilities|GetClass Other))
    (if (not (Variables|HitDelay|GetWasHitRecently))
      (Utilities|FlowControl|Sequence
        (:then_0
          (Variables|HitDelay|SetWasHitRecently true))
        (:then_1
          (Utilities|FlowControl|Delay (Variables|HitDelay|GetHitDelay))
          (Variables|HitDelay|SetWasHitRecently false))
        (:then_2
          (bind _asbp_base_buddy (Utilities|Casting|CastToBP_BaseBuddy Other))
          (Default|BumperForce _asbp_base_buddy (Variables|Default|GetBumperForce) (* HitNormal -1.0))
          (Audio|Components|Audio|Play (Variables|Default|GetSoundFX) 0.0)
          (Default|AddScore (Variables|Default|GetPinballTable) (Variables|Default|GetScoreIncrement)))
        (:then_3
          (Game|SpawnActorfromClass "/Game/VisualFX/BP_ScoreText.BP_ScoreText_C" (Math|Transform|MakeTransform _returnvalue "0, 0,0.000000") "Undefined" 0 1.9 _returnvalue 2e+02 (Variables|Default|GetScoreIncrement) 0))))))

(fn ConstructionScript)