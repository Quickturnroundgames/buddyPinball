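; BP_TippingPointShelf is a shelf that starts sliding back and forth along X on BeginPlay, carrying any buddies on it.
; A timeline's alpha scales a per-frame, delta-time-based offset, and a FlipFlop on finish alternates playback and direction to loop the motion.
; The BuddyOverlap component tracks overlapping BP_BaseBuddy actors, whose meshes receive the same offset, applied in world space while the shelf moves in relative space.
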(event OnComponentBeginOverlap(BuddyOverlap)
  (params (OverlappedComponent :type Primitive%20Component%20Object%20Reference) (OtherActor :type Actor%20Object%20Reference) (OtherComp :type Primitive%20Component%20Object%20Reference) (OtherBodyIndex :type Integer) (bFromSweep :type Boolean) (SweepResult :type Hit%20Result%20Structure%20%28by%20ref%29))
  ;[0 0.1354 1] OVERLAP
  (if (== "/Game/Character/BP_BaseBuddy.BP_BaseBuddy_C" (Utilities|GetClass OtherActor))
    (bind _asbp_base_buddy (Utilities|Casting|CastToBP_BaseBuddy OtherActor))
    (Utilities|Array|Add (Variables|Default|GetoverlappedBuddies) _asbp_base_buddy)))

(event OnComponentEndOverlap(BuddyOverlap)
  (params (OverlappedComponent :type Primitive%20Component%20Object%20Reference) (OtherActor :type Actor%20Object%20Reference) (OtherComp :type Primitive%20Component%20Object%20Reference) (OtherBodyIndex :type Integer))
  ;[0 0.1354 1] OVERLAP
  (if (== "/Game/Character/BP_BaseBuddy.BP_BaseBuddy_C" (Utilities|GetClass OtherActor))
    (bind _asbp_base_buddy (Utilities|Casting|CastToBP_BaseBuddy OtherActor))
    (Utilities|Array|RemoveItem (Variables|Default|GetoverlappedBuddies) _asbp_base_buddy)))

(event Custom|StartMovement
  (bind _returnvalue (Utilities|Time|GetWorldDeltaSeconds))
  ;[0 0.9325 1] MOVEMENT
  (Variables|Default|SetisActive true)
  (bind _movementalpha (Timeline|MovementTimeline Play)
    (:Update
      (if (stale _isa)
        (Utilities|FlowControl|Sequence
          (:then_0
            (Transformation|AddRelativeLocation (Variables|Default|GetTippingPointShelf) (Math|Vector|MakeVector (* _movementalpha (Variables|Default|GetmoveAmount) _returnvalue) 0.0 0.0) true true))
          (:then_1
            (for _array_element (Variables|Default|GetoverlappedBuddies)
              (Transformation|AddWorldOffset (Variables|/Script/Engine.Character|GetMesh _array_element) (Math|Vector|MakeVector (* _movementalpha (Variables|Default|GetmoveAmount) _returnvalue) 0.0 0.0) false true))))
        (else
          (Transformation|AddRelativeLocation (Variables|Default|GetTippingPointShelf) (Math|Vector|MakeVector (* _movementalpha (Variables|Default|GetmoveAmount) -1.0 _returnvalue) 0.0 0.0) true true)
          (for _array_element_2 (Variables|Default|GetoverlappedBuddies)
            (Transformation|AddWorldOffset (Variables|/Script/Engine.Character|GetMesh _array_element_2) (Math|Vector|MakeVector (* _movementalpha (Variables|Default|GetmoveAmount) -1.0 _returnvalue) 0.0 0.0) false true)))))
    (:Finished
      (bind _isa (Utilities|FlowControl|FlipFlop)
        (:A
          (Timeline|MovementTimeline ReverseFromEnd))
        (:B
          (Timeline|MovementTimeline PlayFromStart))))))

(event EventBeginPlay
  (CallFunction|StartMovement))

(event EventTick
  (params (DeltaSeconds :type Float%20%28single-precision%29))
  (if (Variables|Default|GetisActive)
    _))

(fn ConstructionScript)