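; Base buddy character that serves as the ragdoll ball on a pinball table.
; A BuddyState switch gates ragdoll, gauge-spline, portal and points-hole behaviour, toggling physics and capsule size between modes.
; While ragdolled, Tick snaps the shrunken capsule to the hips, caps speed and runs a low-velocity timer.
; Bumpers, nudges and exit launches set body velocities, some adding bone impulses, while timelines drive spline travel and portal shrink, spin and regrow.
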(event Custom|StartFailTimer
  ;[1 1 1] BUDDY STATIC TIMER
  (if (not (Variables|StaticTimer|GetFailTimerCounting))
    (Variables|StaticTimer|SetFailTimerCounting true)
    (Utilities|FlowControl|RetriggerableDelay (Variables|StaticTimer|GetFailTimer))
    (if (and (Utilities|Enum|Equal(Enum) "NewEnumerator1" (Variables|Default|GetbuddyState)) (Variables|StaticTimer|GetFailTimerCounting))
      (Variables|StaticTimer|SetFailTimerCounting false))))

(event EventBeginPlay
  ;[1 0 0] BEGIN PLAY
  (Variables|Portals|SetInitialScale (Transformation|GetActorScale3D))
  (if (Variables|BeginPlay|GetshouldStartAsRagdoll)
    (CallFunction|TurnRagdollON)))

(event EventTick
  (params (DeltaSeconds :type Float%20%28single-precision%29))
  (bind _maxvelocity (Variables|Velocity|GetMaxVelocity))
  (bind _capsulecomponent (Variables|Collision|GetCapsuleComponent))
  (bind _minvelocity (Variables|Velocity|GetMinVelocity))
  ;[1 0 0] EVENT TICK
  (Utilities|FlowControl|Sequence
    (:then_1
      (switch Utilities|FlowControl|Switch|SwitchonEBuddyState (Variables|Default|GetbuddyState)
        (:NewEnumerator1
          (Utilities|FlowControl|Sequence
            (:then_0
              (Transformation|SetWorldLocation _capsulecomponent (Transformation|GetSocketLocation (Variables|Character|GetMesh) "QuickRigCharacter_Hips") false false)
              (Class|PrimitiveComponent|SetAllPhysicsLinearVelocity _capsulecomponent "0, 0, 0" false))
            (:then_1
              (if (< (Math|Vector|VectorLengthSquared (Transformation|GetComponentVelocity (Variables|Character|GetMesh))) (* _minvelocity _minvelocity))
                (CallFunction|StartFailTimer)
                (else
                  (Utilities|FlowControl|Sequence
                    (:then_0
                      (if (Variables|StaticTimer|GetFailTimerCounting)
                        (Variables|StaticTimer|SetFailTimerCounting false)))
                    (:then_1
                      (if (> (Math|Vector|VectorLengthSquared (Transformation|GetComponentVelocity (Variables|Character|GetMesh))) (* _maxvelocity _maxvelocity))
                        (Physics|SetPhysicsLinearVelocity (Variables|Character|GetMesh) (Math|Vector|ClampVectorSize (Transformation|GetComponentVelocity (Variables|Character|GetMesh)) 0.0 (Variables|Velocity|GetMaxVelocity)) false "None")))))))))
        (:NewEnumerator5
          (Transformation|SetWorldLocation (Variables|Collision|GetCapsuleComponent) (Transformation|GetWorldLocation (Variables|Character|GetMesh)) false false))))
    (:then_2
      (Transformation|SetWorldLocation (Variables|Default|GetCentre) (Transformation|GetSocketLocation (Variables|Character|GetMesh) "QuickRigCharacter_Hips") false false))))

(event Custom|ToggleRagdoll
  (switch Utilities|FlowControl|Switch|SwitchonEBuddyState (Variables|Default|GetbuddyState)
    (:NewEnumerator0
      (|RagdollON :!label _label))
    (:NewEnumerator1
      (|RagdollOFF))
    (:NewEnumerator2
      (goto _label))
    (:NewEnumerator3
      (goto _label))))

(event Custom|LaunchFromPinball
  (params (LaunchVel :type Float%20%28single-precision%29))
  (Utilities|FlowControl|Sequence
    (:then_0
      (switch Utilities|FlowControl|Switch|SwitchonEBuddyState (Variables|Default|GetbuddyState)
        (:NewEnumerator0
          (|RagdollON :!label _label))
        (:NewEnumerator1
          (|RagdollOFF))
        (:NewEnumerator2
          (goto _label))
        (:NewEnumerator3
          (goto _label))))
    (:then_1
      (Class|PrimitiveComponent|SetAllPhysicsLinearVelocity (Variables|Character|GetMesh) (Math|Vector|MakeVector 0.0 0.0 LaunchVel) false))))

(event Custom|BumperForce
  (params (BumperForce :type Float%20%28single-precision%29) (ForceDirection :type Vector))
  (bind (_x _y _z) (Math|Vector|BreakVector ForceDirection))
  (bind _returnvalue (Math|Vector|MakeVector 0.0 _y _z))
  (bind _returnvalue_2 (Math|Vector|Normalize _returnvalue))
  (bind _returnvalue_3 (* _returnvalue_2 BumperForce))
  (Class|PrimitiveComponent|SetAllPhysicsLinearVelocity (Variables|Character|GetMesh) _returnvalue_3 false)
  (Physics|AddImpulse (Variables|Character|GetMesh) (* _returnvalue_3 0.6) "QuickRigCharacter_Hips" false))

(event Custom|FollowGaugeSpline
  (params (SplineToFollow :type BP%20Invisible%20Snake%20Follow%20Spline%20Object%20Reference) (MoveSpeed :type Float%20%28single-precision%29) (LaunchForce :type Vector) (ExpellForce :type Float%20%28single-precision%29))
  (bind _returnvalue (* ExpellForce MoveSpeed 3.0))
  (bind _returnvalue_2 (* LaunchForce _returnvalue))
  (switch Utilities|FlowControl|Switch|SwitchonEBuddyState (Variables|Default|GetbuddyState)
    (:NewEnumerator1
      (bind _output_get (Variables|Splines|SetFollowSpline SplineToFollow))
      (Components|Timeline|SetPlayRate (Variables|Default|GetGaugeSplineTimeline) MoveSpeed)
      (Variables|Default|SetbuddyState "NewEnumerator2")
      (Utilities|FlowControl|Sequence
        (:then_0
          (CallFunction|TurnRagdollOFF "NewEnumerator4"))
        (:then_1
          (bind _alpha (Timeline|GaugeSplineTimeline PlayFromStart)
            (:Update
              (Transformation|SetWorldLocationAndRotation (Variables|Collision|GetCapsuleComponent) (Spline|GetLocationatDistanceAlongSpline (Variables|/Game/PinballsBPs/Splines/BP_InvisibleSnakeFollowSpline.BP_InvisibleSnakeFollowSpline_C|GetSpline _output_get) (Math|Float|Lerp 0.0 (Spline|GetSplineLength (Variables|/Game/PinballsBPs/Splines/BP_InvisibleSnakeFollowSpline.BP_InvisibleSnakeFollowSpline_C|GetSpline _output_get)) _alpha) "World") (Math|Conversions|RotationFromXVector (Class|SplineComponent|GetUpVectoratDistanceAlongSpline (Variables|/Game/PinballsBPs/Splines/BP_InvisibleSnakeFollowSpline.BP_InvisibleSnakeFollowSpline_C|GetSpline _output_get) (Math|Float|Lerp 0.0 (Spline|GetSplineLength (Variables|/Game/PinballsBPs/Splines/BP_InvisibleSnakeFollowSpline.BP_InvisibleSnakeFollowSpline_C|GetSpline _output_get)) _alpha) "World")) false true)
              (if (>= _alpha 0.9)
                (Default|PlaySplineEndFX (Variables|Splines|GetFollowSpline))))
            (:Finished
              (CallFunction|TurnRagdollON)
              (Class|PrimitiveComponent|SetAllPhysicsLinearVelocity (Variables|Character|GetMesh) _returnvalue_2 false)
              (Physics|AddImpulse (Variables|Character|GetMesh) (* _returnvalue_2 0.6) "QuickRigCharacter_Hips" false))))))))

(event Custom|NudgeInDirection
  (params (NudgeDirection :type Vector%202D%20Structure))
  (bind (_x _y) (Math|Vector2D|BreakVector2D NudgeDirection))
  (bind _realisticnudge (Variables|Velocity|GetrealisticNudge))
  (bind _nudgeforce (Variables|Velocity|GetNudgeForce))
  (bind _returnvalue (* _y 2.0))
  (bind _returnvalue_2 (Math|Vector|MakeVector 0.0 _x _returnvalue))
  (bind _returnvalue_3 (* _returnvalue_2 _nudgeforce))
  (switch Utilities|FlowControl|Switch|SwitchonEBuddyState (Variables|Default|GetbuddyState)
    (:NewEnumerator1
      (Class|PrimitiveComponent|SetAllPhysicsLinearVelocity (Variables|Character|GetMesh) _returnvalue_3 _realisticnudge)
      (Physics|AddImpulse (Variables|Character|GetMesh) (* _returnvalue_3 0.6) "QuickRigCharacter_Neck" _realisticnudge))))

(event Custom|EnteredPortal
  (params (travelTime :type Float%20%28single-precision%29) (portalEntrance :type BP%20Portal%20Entrance%20Object%20Reference) (portalExitLocation :type Vector) (portalExitSpeed :type Float%20%28single-precision%29) (swapsSide :type Boolean))
  (bind _mesh (Variables|Character|GetMesh))
  (bind _returnvalue (Math|Vector|GetUpVector _mesh))
  (bind (_x _y _z) (Math|Vector|BreakVector _returnvalue))
  (switch Utilities|FlowControl|Switch|SwitchonEBuddyState (Variables|Default|GetbuddyState)
    (:NewEnumerator1
      (Utilities|FlowControl|Sequence
        (:then_0
          (Variables|Default|SetbuddyState "NewEnumerator3")
          (CallFunction|StopRagdollfromMoving))
        (:then_1
          (bind (_direction _shrinkalpha _rotatealpha) (Timeline|ShrinkTimeline PlayFromStart)
            (:Update
              (Transformation|SetWorldScale3D (Variables|Character|GetMesh) (* (Variables|Portals|GetInitialScale) _shrinkalpha))
              (Transformation|SetWorldRotation (Variables|Character|GetMesh) (Math|Rotator|CombineRotators (Math|Rotator|MakeRotator (.Roll (Math|Rotator|BreakRotator (Transformation|GetWorldRotation (Variables|Character|GetMesh)))) 0.0 0.0) (Math|Rotator|MakeRotator (* _rotatealpha (Variables|Portals|GetportalRotateSpeed) (Utilities|Time|GetWorldDeltaSeconds)) 0.0 0.0)) false false)
              (Transformation|SetWorldLocation (Variables|Character|GetMesh) (Math|Interpolation|VInterpTo (Transformation|GetWorldLocation (Variables|Character|GetMesh)) (Transformation|GetWorldLocation (Variables|/Script/Engine.Actor|GetRootComponent portalEntrance)) (Utilities|Time|GetWorldDeltaSeconds) 2.0) false true))
            (:Finished
              (if swapsSide
                (Default|SwapTableSide (Variables|PinballTable|GetpinballTable))
                (Utilities|FlowControl|Delay travelTime)
                (Transformation|SetWorldLocation (Variables|Character|GetMesh) portalExitLocation false true)
                (bind _scaleupalpha (Timeline|ScaleUpTimeline PlayFromStart)
                  (:Update
                    (Transformation|SetWorldScale3D (Variables|Character|GetMesh) (* (Variables|Portals|GetInitialScale) _scaleupalpha))
                    (Transformation|SetWorldRotation (Variables|Character|GetMesh) (Math|Rotator|CombineRotators (Transformation|GetWorldRotation (Variables|Character|GetMesh)) (Math|Rotator|MakeRotator (* (Variables|Portals|GetportalRotateSpeed) (Utilities|Time|GetWorldDeltaSeconds) -1.0) 0.0 0.0)) false false))
                  (:Finished
                    (CallFunction|TurnRagdollON)
                    (Class|PrimitiveComponent|SetAllPhysicsLinearVelocity (Variables|Character|GetMesh) (* (Math|Vector|Normalize (Math|Vector|MakeVector 0.0 _y _z)) portalExitSpeed) false)))))))))))

(event Custom|EnteredPointsHoleArea
  (if (Utilities|Enum|Equal(Enum) (Variables|Default|GetbuddyState) "NewEnumerator1")
    (Utilities|FlowControl|Sequence
      (:then_0
        (Variables|Default|SetbuddyState "NewEnumerator5")
        (CallFunction|StopRagdollfromMoving)))))

(event Custom|LeavePointsHoleArea
  (params (launchDirection :type Vector) (launchForce :type Float%20%28single-precision%29))
  (if (Utilities|Enum|Equal(Enum) (Variables|Default|GetbuddyState) "NewEnumerator5")
    (CallFunction|TurnRagdollON)
    (Class|PrimitiveComponent|SetAllPhysicsLinearVelocity (Variables|Character|GetMesh) (* launchDirection launchForce) false)))

(fn ConstructionScript
  (bind _capsulecomponent (Variables|Collision|GetCapsuleComponent))
  (bind (_outradius _outhalfheight) (Class|CapsuleComponent|GetUnscaledCapsuleSize _capsulecomponent))
  (Variables|Initial|SetInitialCharacterTransform (Transformation|GetRelativeTransform (Variables|Character|GetMesh)))
  (Variables|Initial|SetInitialRadiusHalfHeight (Math|Vector|MakeVector _outradius _outradius _outhalfheight)))

(fn GetCentreWorldLocation
  (return (Transformation|GetWorldLocation (Variables|Default|GetCentre))))

(fn GetIsBeingDragged
  (return false))

(fn GetFeetCapsuleWordLocation
  (return (+ (Transformation|GetWorldLocation (Variables|Collision|GetCapsuleComponent)) (Math|Vector|MakeVector 0.0 0.0 (.Z (Math|Vector|BreakVector (Variables|Initial|GetInitialRadiusHalfHeight)))))))

(fn GetHalfHeight
  (return (.Z (Math|Vector|BreakVector (Variables|Initial|GetInitialRadiusHalfHeight)))))

(fn StopRagdollfromMoving
  (bind _mesh (Variables|Character|GetMesh))
  (bind _capsulecomponent (Variables|Collision|GetCapsuleComponent))
  (bind _mesh_2 (Variables|Character|GetMesh))
  (bind _initialradiushalfheight (Variables|Initial|GetInitialRadiusHalfHeight))
  (bind (_x _y _z) (Math|Vector|BreakVector _initialradiushalfheight))
  (Utilities|FlowControl|Sequence
    (:then_0
      (Variables|Default|SetbuddyState "NewEnumerator5"))
    (:then_1
      (Utilities|FlowControl|Sequence
        (:then_0
          (Physics|SetSimulatePhysics _mesh false)
          (Class|SkeletalMeshComponent|SetPhysicsBlendWeight _mesh 0.0))
        (:then_1
          (Components|Capsule|SetCapsuleRadius _capsulecomponent _x true)
          (Components|Capsule|SetCapsuleHalfHeight _capsulecomponent _z true))))
    (:then_2
      (Physics|SetEnableGravity (Variables|Collision|GetCapsuleComponent) false)
      (Class|PrimitiveComponent|SetAllPhysicsLinearVelocity (Variables|Collision|GetCapsuleComponent) "0, 0, 0" false)
      (Physics|SetEnableGravity _mesh_2 false)
      (Class|PrimitiveComponent|SetAllPhysicsLinearVelocity _mesh_2 "0, 0, 0" false))))

(event Custom|TurnRagdollOFF
  (params (buddyState :type EBuddyState%20Enum :default "NewEnumerator4"))
  (bind _mesh (Variables|Character|GetMesh))
  (bind _mesh_2 (Variables|Character|GetMesh))
  (bind _capsulecomponent (Variables|Collision|GetCapsuleComponent))
  (bind _initialradiushalfheight (Variables|Initial|GetInitialRadiusHalfHeight))
  (bind (_x _y _z) (Math|Vector|BreakVector _initialradiushalfheight))
  (Variables|Default|SetbuddyState buddyState)
  (Utilities|FlowControl|Sequence
    (:then_0
      (Physics|SetSimulatePhysics _mesh false)
      (Class|SkeletalMeshComponent|SetPhysicsBlendWeight _mesh 0.0)
      (Collision|SetCollisionProfileName _mesh_2 "NoCollision" :!class /Script/Engine.PrimitiveComponent)
      (Transformation|AttachComponentToComponent _mesh_2 (Variables|Collision|GetCapsuleComponent) "None" "SnapToTarget" "SnapToTarget" "SnapToTarget" true))
    (:then_1
      (Transformation|SetRelativeTransform (Variables|Character|GetMesh) (Variables|Initial|GetInitialCharacterTransform) false false)
      (Components|Capsule|SetCapsuleRadius _capsulecomponent _x true)
      (Components|Capsule|SetCapsuleHalfHeight _capsulecomponent _z true)
      (Collision|SetCollisionProfileName (Variables|Character|GetMesh) "Ragdoll" :!class /Script/Engine.PrimitiveComponent))))

(event Custom|TurnRagdollON
  (bind _returnvalue (Utilities|Name|MakeLiteralName "QuickRigCharacter_Hips"))
  (bind _mesh (Variables|Character|GetMesh))
  (bind _capsulecomponent (Variables|Collision|GetCapsuleComponent))
  (bind _mesh_2 (Variables|Character|GetMesh))
  (Utilities|FlowControl|Sequence
    (:then_0
      (Utilities|FlowControl|Sequence
        (:then_0
          (Collision|SetCollisionProfileName _mesh "Ragdoll" :!class /Script/Engine.PrimitiveComponent)
          (Class|SkeletalMeshComponent|SetAllBodiesBelowSimulatePhysics (Variables|Character|GetMesh) _returnvalue true true)
          (Class|SkeletalMeshComponent|SetAllBodiesBelowPhysicsBlendWeight _mesh _returnvalue 1.0 false true)
          (Physics|SetEnableGravity (Variables|Character|GetMesh) true))
        (:then_1
          (Physics|AddImpulseatLocation _mesh_2 "0, 0,-30.000000" "0, 0, 0" "QuickRigCharacter_RightForeArm")
          (Physics|AddImpulseatLocation _mesh_2 "0, 0,-30.000000" "0, 0, 0" "QuickRigCharacter_LeftForeArm"))
        (:then_2
          (Components|Capsule|SetCapsuleRadius _capsulecomponent 1.0 true)
          (Components|Capsule|SetCapsuleHalfHeight _capsulecomponent 1.0 true))))
    (:then_1
      (Variables|Default|SetbuddyState "NewEnumerator1"))))